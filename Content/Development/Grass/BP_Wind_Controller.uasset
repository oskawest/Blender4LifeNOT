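; Wind controller actor that feeds global foliage wind data to materials through the PC_Global_Foliage_Wind parameter collection.
; Each tick it flattens and normalizes the vector between its Start and End components to set the wind direction, plus a far-scaled copy as the wind target.
; It also writes the first player pawn's location every tick.
; A Wind_Strength update exists but is disconnected and never runs.
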(event `self.ReceiveTick`
  (params (DeltaSeconds :type "Float (single-precision)"))
  (bind (_x _y) (`KismetMathLibrary.BreakVector2D` (`KismetMathLibrary.Normal2D` (`KismetMathLibrary.MakeVector2D` (.x (- (`SceneComponent.K2_GetComponentLocation` (`self.end`)) (`SceneComponent.K2_GetComponentLocation` (`self.start`)))) (.y (- (`SceneComponent.K2_GetComponentLocation` (`self.end`)) (`SceneComponent.K2_GetComponentLocation` (`self.start`))))))))
  (bind _returnvalue (`KismetMathLibrary.MakeVector` _x _y))
  ;[1 1 1] Wind Direction
  (`KismetMaterialLibrary.SetVectorParameterValue` "/Game/Development/Grass/PC_Global_Foliage_Wind.PC_Global_Foliage_Wind" "WindDirection" (`KismetMathLibrary.Conv_VectorToLinearColor` _returnvalue))
  (`KismetMaterialLibrary.SetVectorParameterValue` "/Game/Development/Grass/PC_Global_Foliage_Wind.PC_Global_Foliage_Wind" "Wind_Target" (`KismetMathLibrary.Conv_VectorToLinearColor` (* _returnvalue 50000.0)))
  (`KismetMaterialLibrary.SetVectorParameterValue` "/Game/Development/Grass/PC_Global_Foliage_Wind.PC_Global_Foliage_Wind" "Player_Position" (`KismetMathLibrary.Conv_VectorToLinearColor` (`self.K2_GetActorLocation` (`GameplayStatics.GetPlayerPawn` 0)))))

(fn `UserConstructionScript`)