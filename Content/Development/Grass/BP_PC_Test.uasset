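; Test Blueprint, apparently for driving a material parameter collection on a plane.
; BeginPlay creates a dynamic instance of M_MaterialExpression_Test on the plane, stores it unused, and builds an array of indexed "Scalar" parameter names.
; A disconnected node would write a time-based cosine wave, remapped to 0–1, into the first named parameter of PC_Wind_RunTime_Variables.
; Tick is empty, so nothing animates at runtime.
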(event `self.ReceiveBeginPlay`
  (bind _returnvalue (`PrimitiveComponent.CreateDynamicMaterialInstance` (`self.Plane`) 0 "/Game/Development/Grass/M_MaterialExpression_Test.M_MaterialExpression_Test" "None"))
  (set `self.MDI_Material` _returnvalue)
  (for _index (range 2)
    (`KismetArrayLibrary.Array_Set` (`self.Parameters`) _index (`KismetStringLibrary.Conv_StringToName` (`KismetStringLibrary.Concat_StrStr` "Scalar" (`KismetStringLibrary.Conv_IntToString` _index))) true)))

(event `self.ReceiveTick`
  (params (DeltaSeconds :type "Float (single-precision)")))

(fn `UserConstructionScript`)