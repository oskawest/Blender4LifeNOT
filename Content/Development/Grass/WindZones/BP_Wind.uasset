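; BP_Wind is a grass wind zone actor that moves a wind point along a spline path.
; Each Tick it sets the timeline play rate from FSpeed and plays it, mapping the ConstantWind track to distance along SplineWindPath.
; The timeline update moves SMWindLocation to that point and stores it as VWindPosition.
; It derives VWindDirection by normalizing the change from the previous position.
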(event `self.ReceiveTick`
  (params (DeltaSeconds :type "Float (single-precision)"))
  (bind _spline_wind_path (`self.Spline_Wind_Path`))
  (`TimelineComponent.SetPlayRate` (`self.Timeline_0`) (`self.fSpeed`))
  (bind (_direction _constantwind) (`Timeline|Timeline_0`)
    (:`Update`
      (bind _returnvalue (`SplineComponent.GetLocationAtDistanceAlongSpline` _spline_wind_path (* _constantwind (`SplineComponent.GetSplineLength` _spline_wind_path)) "World"))
      (`SceneComponent.K2_SetWorldLocation` (`self.SM_Wind_Location`) _returnvalue false false)
      (bind _output_get (set `self.vWindPosition` _returnvalue))
      (set `self.vWindDirection` (`KismetMathLibrary.Normal` (- _output_get (`self.vWindPositionOld`))))
      (set `self.vWindPositionOld` (`self.vWindPosition`)))))

(fn `UserConstructionScript`)