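; Wind controller that feeds global wind direction and player position to foliage materials and paints local wind zones into a render target.
; Each tick it gathers "Wind"-tagged BP_Wind actors and traces down from each to find a collision UV.
; Hits route through point damage on itself, stamping that wind's direction, size and strength.
; A second target holds a copy, shifted by player movement with a subtract material to remove strength.
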(event `self.ReceiveBeginPlay`
  (bind _rt_wind_2 (`self.RT_Wind_2`))
  (`self.EnableInput` (`GameplayStatics.GetPlayerController` 0))
  (`KismetRenderingLibrary.ClearRenderTarget2D` (`self.RT_Wind_1`))
  (`MaterialInstanceDynamic.SetTextureParameterValue` (`self.DMI_Wind_Draw_Copy`) "Texture_To_Copy" "/Game/Development/Grass/WindZones/RT_WindZones.RT_WindZones")
  (`KismetRenderingLibrary.ClearRenderTarget2D` _rt_wind_2)
  (`MaterialInstanceDynamic.SetTextureParameterValue` (`self.DMI_Wind_Draw`) "Subtraction" _rt_wind_2)
  (`MaterialInstanceDynamic.SetTextureParameterValue` (`self.DMI_Wind_Move_Subtract`) "T_WindZones" "/Game/Development/Grass/WindZones/RT_WindZones.RT_WindZones")
  (set `self.V_Player_Pos_Old` (`self.K2_GetActorLocation` (`GameplayStatics.GetPlayerPawn` 0))))

(event `self.ReceiveTick`
  (params (DeltaSeconds :type "Float (single-precision)"))
  (bind _v_player_pos (`self.V_Player_Pos`))
  (bind _dmi_wind_draw (`self.DMI_Wind_Draw`))
  (bind (_x _y) (`KismetMathLibrary.BreakVector2D` (`KismetMathLibrary.Normal2D` (`KismetMathLibrary.MakeVector2D` (.x (- (`SceneComponent.K2_GetComponentLocation` (`self.end`)) (`SceneComponent.K2_GetComponentLocation` (`self.start`)))) (.y (- (`SceneComponent.K2_GetComponentLocation` (`self.end`)) (`SceneComponent.K2_GetComponentLocation` (`self.start`))))))))
  (bind _returnvalue (`KismetMathLibrary.MakeVector` _x _y))
  (`KismetMaterialLibrary.SetVectorParameterValue` "/Game/Development/Grass/PC_Global_Foliage_Wind.PC_Global_Foliage_Wind" "WindDirection" (`KismetMathLibrary.Conv_VectorToLinearColor` _returnvalue))
  (`KismetMaterialLibrary.SetVectorParameterValue` "/Game/Development/Grass/PC_Global_Foliage_Wind.PC_Global_Foliage_Wind" "Wind_Target" (`KismetMathLibrary.Conv_VectorToLinearColor` (* _returnvalue 500000.0)))
  (bind _outactors (`GameplayStatics.GetAllActorsWithTag` "PlayerTest"))
  (bind _output_get (set `self.V_Player_Pos` (`self.K2_GetActorLocation` (`GameplayStatics.GetPlayerPawn` 0))))
  (`KismetMaterialLibrary.SetVectorParameterValue` "/Game/Development/Grass/PC_Global_Foliage_Wind.PC_Global_Foliage_Wind" "Player_Position" (`KismetMathLibrary.Conv_VectorToLinearColor` _output_get))
  (`KismetArrayLibrary.Array_Clear` (`self.V_Wind_Positions`))
  (`KismetArrayLibrary.Array_Clear` (`self.V_Wind_Directions`))
  (`KismetArrayLibrary.Array_Clear` (`self.vWindStrengths`))
  (`KismetArrayLibrary.Array_Clear` (`self.vWindSizes`))
  (bind _outactors_2 (`GameplayStatics.GetAllActorsWithTag` "Wind"))
  (for _array_element _outactors_2
    (bind _asbp_wind (cast `/Game/Development/Grass/WindZones/BP_Wind` _array_element))
    (`KismetArrayLibrary.Array_Add` (`self.V_Wind_Positions`) (`/Game/Development/Grass/WindZones/BP_Wind.vWindPosition` _asbp_wind))
    (`KismetArrayLibrary.Array_Add` (`self.V_Wind_Directions`) (`self.vector RG ( -1 to 1, -> 0 to 1)` (`/Game/Development/Grass/WindZones/BP_Wind.vWindDirection` _asbp_wind)))
    (`KismetArrayLibrary.Array_Add` (`self.vWindStrengths`) (`/Game/Development/Grass/WindZones/BP_Wind.fWindStrength` _asbp_wind))
    (`KismetArrayLibrary.Array_Add` (`self.vWindSizes`) (`/Game/Development/Grass/WindZones/BP_Wind.fWindSize` _asbp_wind)))
  (for _array_element_2 (`self.V_Wind_Positions`)
    (bind (_outhit _returnvalue_2) (`KismetSystemLibrary.LineTraceSingle` :`Start` _array_element_2 :`End` (- _array_element_2 (0.0 0.0 20000.0)) :`TraceChannel` "TraceTypeQuery3" :`bTraceComplex` true :`bIgnoreSelf` false :`DrawTime` 0.5))
    (if _returnvalue_2
      (bind (_bblockinghit _binitialoverlap _time _distance _location _impactpoint _normal _impactnormal _physmat _hitactor) (`GameplayStatics.BreakHitResult` _outhit))
      (`/Engine/EditorBlueprintResources/StandardMacros.IsValid` _hitactor
        (:`Is Valid`
          (set `self.Collision UV Hit` (`GameplayStatics.FindCollisionUV` _outhit))
          (`GameplayStatics.ApplyPointDamage` self 100.0 (`KismetMathLibrary.MakeVector` 0.0 0.0 1.0) _outhit null _hitactor)))))
  (`MaterialInstanceDynamic.SetScalarParameterValue` _dmi_wind_draw "ForceStrength" 0.0)
  (`MaterialInstanceDynamic.SetVectorParameterValue` :`self` _dmi_wind_draw :`ParameterName` "WindDirection")
  (`KismetRenderingLibrary.DrawMaterialToRenderTarget` "/Game/Development/Grass/WindZones/RT_WindZones.RT_WindZones" _dmi_wind_draw)
  (`MaterialInstanceDynamic.SetScalarParameterValue` _dmi_wind_draw "ForceStrength" 3.0)
  (bind _returnvalue_3 (`KismetMaterialLibrary.GetScalarParameterValue` "/Game/Development/Grass/PC_Global_Foliage_Wind.PC_Global_Foliage_Wind" "Dynamic_Wind_Distance"))
  (`MaterialInstanceDynamic.SetVectorParameterValue` (`self.DMI_Wind_Draw_Copy`) "MoveRT" (`KismetMathLibrary.Conv_VectorToLinearColor` (/ (- (`self.V_Player_Pos_Old`) _v_player_pos) _returnvalue_3)))
  (`MaterialInstanceDynamic.SetVectorParameterValue` (`self.DMI_Wind_Move_Subtract`) "MoveRT" (`KismetMathLibrary.Conv_VectorToLinearColor` (/ (- (`self.V_Player_Pos_Old`) _v_player_pos) _returnvalue_3)))
  (`KismetRenderingLibrary.DrawMaterialToRenderTarget` (`self.RT_Wind_2`) (`self.DMI_Wind_Move_Subtract`))
  (set `self.V_Player_Pos_Old` _v_player_pos))

(event `Key|One`
  (params (Key :type "Key Structure"))
  (:`Pressed`
    (set `self.V_Wind_Positions` (`|MakeArray` (6000.0 0.0 500.0) :!type "Vector Structure"))))

(event `self.ReceivePointDamage`
  (params (Damage :type "Float (single-precision)") (DamageType :type "DamageType Object Reference") (HitLocation :type "Vector Structure") (HitNormal :type "Vector Structure") (HitComponent :type "PrimitiveComponent Object Reference") (BoneName :type Name) (ShotFromDirection :type "Vector Structure") (InstigatedBy :type "Controller Object Reference") (DamageCauser :type "Actor Object Reference") (HitInfo :type "HitResult Structure (by ref)"))
  (bind _dmi_wind_draw (`self.DMI_Wind_Draw`))
  (`MaterialInstanceDynamic.SetVectorParameterValue` _dmi_wind_draw "WindPosition" (`KismetMathLibrary.Conv_VectorToLinearColor` (`KismetMathLibrary.Conv_Vector2DToVector` (`self.Collision UV Hit`))))
  (for (_array_element _array_index) (`self.V_Wind_Positions`)
    (`self.Compare Vectors` (`.TraceStart` (`GameplayStatics.BreakHitResult` HitInfo)) _array_element
      (:`==`
        (`MaterialInstanceDynamic.SetVectorParameterValue` _dmi_wind_draw "WindDirection" (`KismetMathLibrary.Conv_VectorToLinearColor` (`|GetArrayItem` (`self.V_Wind_Directions`) _array_index)))
        (bind _returnvalue (`KismetMaterialLibrary.GetScalarParameterValue` "/Game/Development/Grass/PC_Global_Foliage_Wind.PC_Global_Foliage_Wind" "Dynamic_Wind_Distance"))
        (`MaterialInstanceDynamic.SetScalarParameterValue` _dmi_wind_draw "ForceSize" (/ (`|GetArrayItem` (`self.vWindSizes`) _array_index) (* _returnvalue 0.01)))
        (`MaterialInstanceDynamic.SetScalarParameterValue` _dmi_wind_draw "ForceStrength" (`|GetArrayItem` (`self.vWindStrengths`) _array_index)))))
  (`KismetRenderingLibrary.DrawMaterialToRenderTarget` "/Game/Development/Grass/WindZones/RT_WindZones.RT_WindZones" _dmi_wind_draw)
  (`KismetRenderingLibrary.DrawMaterialToRenderTarget` (`self.RT_Wind_2`) (`self.DMI_Wind_Draw_Copy`)))

(fn `UserConstructionScript`
  (bind _i_wind_rt_resolution (`self.I_Wind_RT_Resolution`))
  (bind _returnvalue (`KismetRenderingLibrary.CreateRenderTarget2D` _i_wind_rt_resolution _i_wind_rt_resolution))
  (set `self.RT_Wind_1` _returnvalue)
  (bind _returnvalue_2 (`KismetRenderingLibrary.CreateRenderTarget2D` _i_wind_rt_resolution _i_wind_rt_resolution))
  (set `self.RT_Wind_2` _returnvalue_2)
  (bind _returnvalue_3 (`KismetMaterialLibrary.CreateDynamicMaterialInstance` "/Game/Development/Grass/WindZones/M_Wind_Draw_Copy.M_Wind_Draw_Copy" "DMI_Wind_Draw_Copy"))
  (set `self.DMI_Wind_Draw_Copy` _returnvalue_3)
  (bind _returnvalue_4 (`KismetMaterialLibrary.CreateDynamicMaterialInstance` "/Game/Development/Grass/WindZones/M_Wind_Move_Subtract.M_Wind_Move_Subtract" "DMI_Wind_Move_Subtract"))
  (set `self.DMI_Wind_Move_Subtract` _returnvalue_4)
  (bind _returnvalue_5 (`KismetMaterialLibrary.CreateDynamicMaterialInstance` "/Game/Development/Grass/WindZones/M_Wind_Draw_Directional.M_Wind_Draw_Directional" "DMI_Wind_Draw"))
  (set `self.DMI_Wind_Draw` _returnvalue_5))