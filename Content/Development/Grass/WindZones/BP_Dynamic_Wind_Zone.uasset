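; Wind zone actor that paints moving gust positions and their directions into render targets, apparently for grass wind.
; Each tick it shifts wind points along negative X, encodes their direction as color and traces downward, sending point damage to hit actors.
; Its damage event stamps the hit UV and matched direction through a draw material, then ping-pongs render targets through a subtraction material to erase zones over time.
; Key 1 resets the points.
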(event `self.ReceiveBeginPlay`
  (bind _rt_wind_zones_subtraction (`self.RT_Wind_Zones_Subtraction`))
  (`self.EnableInput` (`GameplayStatics.GetPlayerController` 0))
  (`|ExecutionSequence`
    (:`then_0`
      (`KismetRenderingLibrary.ClearRenderTarget2D` (`self.RT_Wind_Zones`))
      (`MaterialInstanceDynamic.SetTextureParameterValue` (`self.MI_Wind_Zones`) "T_WindZones" "/Game/Development/Grass/WindZones/RT_WindZones.RT_WindZones"))
    (:`then_1`
      (`KismetRenderingLibrary.ClearRenderTarget2D` (`self.RT_Wind_Zones_Subtraction`))
      (`MaterialInstanceDynamic.SetTextureParameterValue` (`self.MI_Wind_Zone_Subtraction`) "T_WindZones" _rt_wind_zones_subtraction))
    (:`then_2`
      (`MaterialInstanceDynamic.SetTextureParameterValue` (`self.MI_Wind_Draw_Zone`) "Subtraction" _rt_wind_zones_subtraction))))

(event `self.ReceiveTick`
  (params (DeltaSeconds :type "Float (single-precision)"))
  (bind _windpositions (`self.WindPositions`))
  (for (_array_element _array_index) _windpositions
    (bind _returnvalue (- _array_element (`KismetMathLibrary.MakeVector` (`self.WindSpeed`))))
    (`KismetArrayLibrary.Array_Set` _windpositions _array_index _returnvalue)
    (`KismetArrayLibrary.Array_Set` (`self.WindDirections`) _array_index (`KismetMathLibrary.MakeVector` (* (+ (.x (`KismetMathLibrary.Normal` (- _returnvalue _array_element))) 1.0) 0.5) (* (+ (.y (`KismetMathLibrary.Normal` (- _returnvalue _array_element))) 1.0) 0.5)) true))
  (for _array_element_2 _windpositions
    (bind (_outhit _returnvalue_2) (`KismetSystemLibrary.LineTraceSingle` :`Start` _array_element_2 :`End` (- _array_element_2 (0.0 0.0 2000.0)) :`TraceChannel` "TraceTypeQuery3" :`bTraceComplex` true :`bIgnoreSelf` false))
    (if _returnvalue_2
      (bind (_bblockinghit _binitialoverlap _time _distance _location _impactpoint _normal _impactnormal _physmat _hitactor) (`GameplayStatics.BreakHitResult` _outhit))
      (`/Engine/EditorBlueprintResources/StandardMacros.IsValid` _hitactor
        (:`Is Valid`
          (set `self.Collision UV Hit` (`GameplayStatics.FindCollisionUV` _outhit))
          (`GameplayStatics.ApplyPointDamage` _hitactor 100.0 (`KismetMathLibrary.MakeVector` 0.0 0.0 1.0) _outhit null self))))))

(event `Key|One`
  (params (Key :type "Key Structure"))
  (:`Pressed`
    (set `self.WindPositions` (`|MakeArray` (6000.0 500.0 500.0) (6000.0 6000.0 500.0) :!type "Vector Structure"))))

(event `self.ReceivePointDamage`
  (params (Damage :type "Float (single-precision)") (DamageType :type "DamageType Object Reference") (HitLocation :type "Vector Structure") (HitNormal :type "Vector Structure") (HitComponent :type "PrimitiveComponent Object Reference") (BoneName :type Name) (ShotFromDirection :type "Vector Structure") (InstigatedBy :type "Controller Object Reference") (DamageCauser :type "Actor Object Reference") (HitInfo :type "HitResult Structure (by ref)"))
  (bind _mi_wind_draw_zone (`self.MI_Wind_Draw_Zone`))
  (`MaterialInstanceDynamic.SetVectorParameterValue` _mi_wind_draw_zone "WindPosition" (`KismetMathLibrary.Conv_VectorToLinearColor` (`KismetMathLibrary.Conv_Vector2DToVector` (`self.Collision UV Hit`))))
  (for (_array_element _array_index) (`self.WindPositions`)
    (`/Engine/EditorBlueprintResources/StandardMacros.CompareFloat` (.x _array_element) (.x (`.TraceStart` (`GameplayStatics.BreakHitResult` HitInfo)))
      (:`==`
        (`/Engine/EditorBlueprintResources/StandardMacros.CompareFloat` (.y _array_element) (.y (`.TraceStart` (`GameplayStatics.BreakHitResult` HitInfo)))
          (:`==`
            (`/Engine/EditorBlueprintResources/StandardMacros.CompareFloat` (.z _array_element) (.z (`.TraceStart` (`GameplayStatics.BreakHitResult` HitInfo)))
              (:`==`
                (`MaterialInstanceDynamic.SetVectorParameterValue` _mi_wind_draw_zone "WindDirection" (`KismetMathLibrary.Conv_VectorToLinearColor` (`|GetArrayItem` (`self.WindDirections`) _array_index))))))))))
  (`KismetRenderingLibrary.DrawMaterialToRenderTarget` "/Game/Development/Grass/WindZones/RT_WindZones.RT_WindZones" _mi_wind_draw_zone)
  (`KismetRenderingLibrary.DrawMaterialToRenderTarget` (`self.RT_Wind_Zones_Subtraction`) (`self.MI_Wind_Zones`))
  (`KismetRenderingLibrary.DrawMaterialToRenderTarget` "/Game/Development/Grass/WindZones/RT_WindZones.RT_WindZones" (`self.MI_Wind_Zone_Subtraction`)))

(fn `UserConstructionScript`
  (bind _i_width (`self.I_Width`))
  (bind _i_height (`self.I_Height`))
  (`|ExecutionSequence`
    (:`then_0`
      (bind _returnvalue (`KismetRenderingLibrary.CreateRenderTarget2D` _i_width _i_height "RTF_RGBA8"))
      (set `self.RT_Wind_Zones` _returnvalue)
      (bind _returnvalue_2 (`KismetMaterialLibrary.CreateDynamicMaterialInstance` "/Game/Development/Grass/WindZones/M_Wind_Zones.M_Wind_Zones" "WindZones"))
      (bind _output_get (set `self.MI_Wind_Zones` _returnvalue_2))
      (bind _returnvalue_3 (`KismetMaterialLibrary.CreateDynamicMaterialInstance` "/Game/Development/Grass/WindZones/M_Wind_Draw_Zone.M_Wind_Draw_Zone" "DrawZone"))
      (set `self.MI_Wind_Draw_Zone` _returnvalue_3)
      (bind _returnvalue_4 (`KismetMaterialLibrary.CreateDynamicMaterialInstance` "/Game/Development/Grass/WindZones/M_Wind_Subtraction.M_Wind_Subtraction" "EraseZoneByTime"))
      (bind _output_get_2 (set `self.MI_Wind_Zone_Subtraction` _returnvalue_4))
      (`PrimitiveComponent.SetMaterial` (`self.StaticMeshComponent`) 0 _output_get_2)
      (set `self.WindPositions` (`|MakeArray` (6000.0 500.0 500.0) (6000.0 6000.0 500.0) :!type "Vector Structure")))
    (:`then_1`
      (bind _returnvalue_5 (`KismetRenderingLibrary.CreateRenderTarget2D` _i_width _i_height "RTF_RGBA8"))
      (set `self.RT_Wind_Zones_Subtraction` _returnvalue_5))))